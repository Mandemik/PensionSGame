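; Interactable fuse box that lets the player cut the power during what appears to be a home break-in scenario.
; Overlap with a Character-tagged component shows a yes or no prompt based on ShouldShutOff; yes opens a Tick gate polling Enter.
; Pressing Enter zeroes listed lights, destroys listed actors, briefly shows a broken-box widget, disables Tick and sets Crowed2Distracted on HomeBreakIn_BP.
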(event `self.ReceiveTick`
  (params (DeltaSeconds :type "Float (single-precision)"))
  (`/Engine/EditorBlueprintResources/StandardMacros.Gate` true :!label _label
    (:`Exit`
      (if (`PlayerController.WasInputKeyJustPressed` (`GameplayStatics.GetPlayerController` 0) "Enter")
        (`|ExecutionSequence`
          (:`then_0`
            ;[1 1 1] Comment
            (for _array_element (`self.Lights`)
              (`LightComponent.SetIntensity` (`Light.LightComponent` _array_element) 0.0)))
          (:`then_1`
            (for _array_element_2 (`self.Actors`)
              (`self.K2_DestroyActor` _array_element_2)))
          (:`then_2`
            (bind _returnvalue (`|CreateWidget` "/Game/1Main/Blueprints/Widgets/People/FuseBoxBroke.FuseBoxBroke_C"))
            (`UserWidget.AddToViewport` _returnvalue 0)
            (`KismetSystemLibrary.Delay` 5.0)
            (bind _foundwidgets (`WidgetBlueprintLibrary.GetAllWidgetsOfClass` "/Game/1Main/Blueprints/Widgets/People/FuseBoxBroke.FuseBoxBroke_C"))
            (`Widget.RemoveFromParent` (`|GetArrayItem` _foundwidgets)))
          (:`then_4`
            (`self.SetActorTickEnabled` false)
            (set `self.PowerShutOff` false))
          (:`then_5`
            (bind _outactors (`GameplayStatics.GetAllActorsOfClass` "/Game/1Main/Blueprints/HomeBreakIn_BP.HomeBreakIn_BP_C"))
            (set `/Game/1Main/Blueprints/HomeBreakIn_BP.Crowed2Distracted` true (`|GetArrayItem` _outactors))))))))

(event `self.Box.OnComponentBeginOverlap`
  (params (OverlappedComponent :type "PrimitiveComponent Object Reference") (OtherActor :type "Actor Object Reference") (OtherComp :type "PrimitiveComponent Object Reference") (OtherBodyIndex :type Integer) (bFromSweep :type Boolean) (SweepResult :type "HitResult Structure (by ref)"))
  (if (`self.PowerShutOff`)
    _
    (elif (`ActorComponent.ComponentHasTag` OtherComp "Character")
      (if (`self.ShouldShutOff`)
        (bind _returnvalue (`|CreateWidget` (`self.FuseBox_Yes`)))
        (`UserWidget.AddToViewport` _returnvalue 0)
        (goto _label :!via `Open`)
        (else
          (bind _returnvalue_2 (`|CreateWidget` (`self.FuseBox_No`)))
          (`UserWidget.AddToViewport` _returnvalue_2 0))))))

(event `self.Box.OnComponentEndOverlap`
  (params (OverlappedComponent :type "PrimitiveComponent Object Reference") (OtherActor :type "Actor Object Reference") (OtherComp :type "PrimitiveComponent Object Reference") (OtherBodyIndex :type Integer))
  (if (`self.PowerShutOff`)
    _
    (elif (`ActorComponent.ComponentHasTag` OtherComp "Character")
      (bind _foundwidgets (`WidgetBlueprintLibrary.GetAllWidgetsOfClass` (`self.FuseBox_Yes`)))
      (if (> (`KismetArrayLibrary.Array_Length` _foundwidgets) 0)
        (`Widget.RemoveFromParent` (`|GetArrayItem` _foundwidgets))
        (goto _label :!via `Close`))
      (else
        (bind _foundwidgets_2 (`WidgetBlueprintLibrary.GetAllWidgetsOfClass` (`self.FuseBox_No`)))
        (if (> (`KismetArrayLibrary.Array_Length` _foundwidgets_2) 0)
          (`Widget.RemoveFromParent` (`|GetArrayItem` _foundwidgets_2)))))))

(event `self.ReceiveBeginPlay`)

(fn `UserConstructionScript`)