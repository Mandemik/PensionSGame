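; EndMission_BP is a mission-end trigger volume that returns the game to the StartScreen level once the target has been assassinated.
; When a component tagged Character begins overlapping its Box, it checks IsTargetAssassinated and opens that level if true.
; When such a component leaves the Box, it removes the first top-level AssassinateTarget widget found, though this Blueprint never creates that widget.
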(event `self.Box.OnComponentBeginOverlap`
  (params (OverlappedComponent :type "PrimitiveComponent Object Reference") (OtherActor :type "Actor Object Reference") (OtherComp :type "PrimitiveComponent Object Reference") (OtherBodyIndex :type Integer) (bFromSweep :type Boolean) (SweepResult :type "HitResult Structure (by ref)"))
  (if (`ActorComponent.ComponentHasTag` OtherComp "Character")
    (if (`self.IsTargetAssassinated`)
      (`GameplayStatics.OpenLevel` "StartScreen"))))

(event `self.Box.OnComponentEndOverlap`
  (params (OverlappedComponent :type "PrimitiveComponent Object Reference") (OtherActor :type "Actor Object Reference") (OtherComp :type "PrimitiveComponent Object Reference") (OtherBodyIndex :type Integer))
  (if (`ActorComponent.ComponentHasTag` OtherComp "Character")
    (bind _foundwidgets (`WidgetBlueprintLibrary.GetAllWidgetsOfClass` "/Game/1Main/Blueprints/Widgets/Player/AssassinateTarget.AssassinateTarget_C"))
    (`Widget.RemoveFromParent` (`|GetArrayItem` _foundwidgets))))

(fn `UserConstructionScript`)