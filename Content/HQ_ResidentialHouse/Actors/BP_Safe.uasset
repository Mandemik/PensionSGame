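; BP_Safe is an interactive keypad safe that opens when the player enters the correct four-digit code.
; Interacting toggles a long-interact view at CameraRoot through MannequinCharacter, along with actor input and the prompt's visibility.
; Clicks trace under the cursor for CodeButton-tagged components, whose object names are appended as the typed digits.
; A match turns the light green and swings the door on a timeline, while a mismatch clears the entry and turns it red.
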(event `DoorSwitch`
  (`|ExecutionSequence`
    (:`then_0`
      (`LightComponent.SetLightColor` (`self.PointLight`) (struct :`R` 0.029035 :`G` 0.28125 :`A` 1.0) true))
    (:`then_1`
      (bind (_direction _rotation) (`Timeline|DoorOpening`)
        (:`Update`
          (`SceneComponent.K2_SetRelativeRotation` (`self.Safe_Door`) (`KismetMathLibrary.MakeRotator` 0.0 0.0 _rotation) false false))))))

(event `self.Interactable.InteractDelegate`
  (bind _isplayerinteract (`self.IsPlayerInteract`))
  (bind _asmannequin_character (cast `/Game/AdvancedLocomotionV3/Blueprints/MannequinCharacter` (`GameplayStatics.GetPlayerPawn` 0) :!pure true))
  (if (`self.IsPlayerInteract`)
    (`/Game/AdvancedLocomotionV3/Blueprints/ALS_BaseCharacter.SetALS_LongInteractEvent` :`self` _asmannequin_character)
    (`self.DisableInput` self (`GameplayStatics.GetPlayerController` 0))
    (else
      (`/Game/AdvancedLocomotionV3/Blueprints/ALS_BaseCharacter.SetALS_LongInteractEvent` _asmannequin_character true (`SceneComponent.K2_GetComponentToWorld` (`self.CameraRoot`)))
      (`self.EnableInput` self (`GameplayStatics.GetPlayerController` 0))))
  (`SceneComponent.SetVisibility` (`self.Interactable`) _isplayerinteract true)
  (set `self.IsPlayerInteract` (not _isplayerinteract)))

(event `Key|LeftMouseButton`
  (params (Key :type "Key Structure"))
  (bind (_hitresult _returnvalue) (`PlayerController.GetHitResultUnderCursorForObjects` (`GameplayStatics.GetPlayerController` 0) (`|MakeArray` "ObjectTypeQuery1" :!type "EObjectTypeQuery Enum") true))
  (bind (_bblockinghit _binitialoverlap _time _distance _location _impactpoint _normal _impactnormal _physmat _hitactor _hitcomponent) (`GameplayStatics.BreakHitResult` _hitresult))
  (:`Pressed`
    (if _returnvalue
      (if (`ActorComponent.ComponentHasTag` _hitcomponent "CodeButton")
        (`self.InputCode` (`KismetSystemLibrary.GetObjectName` _hitcomponent))))))

(fn `InputCode`
  (params (Number :type String))
  (`LightComponent.SetLightColor` (`self.PointLight`) (struct :`R` 0.141176 :`G` 0.513726 :`B` 1.0 :`A` 1.0) true)
  (bind _output_get (set `self.CurrentCODE` (`KismetStringLibrary.Concat_StrStr` (`self.CurrentCODE`) Number)))
  (if (== (`KismetStringLibrary.Len` _output_get) 4)
    (if (`KismetStringLibrary.EqualEqual_StrStr` (`self.CODE`) (`self.CurrentCODE`))
      (`self.DoorSwitch`)
      (else
        (set `self.CurrentCODE` "")
        (`LightComponent.SetLightColor` (`self.PointLight`) (struct :`R` 0.489583 :`G` 0.014163 :`A` 1.0) true)))))

(fn `UserConstructionScript`)