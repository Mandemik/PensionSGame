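; Interactable intercom keypad that the player uses through a close-up camera.
; Interacting or pressing Use toggles the player character's custom camera at CameraRoot, hands input between character and intercom, and hides or shows the Interactable.
; Left clicks trace under the cursor for CodeButton-tagged components and pass their names to InputCode.
; InputCode and DoorSwitch are empty; the code-check, light and safe-door logic is disconnected.
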(event `self.Interactable.InteractDelegate`
  (`self.InteractWithObject`))

(event `DoorSwitch`)

(event `InteractWithObject`
  (bind _returnvalue (`GameplayStatics.GetPlayerController` 0))
  (bind _returnvalue_2 (`GameplayStatics.GetPlayerController` 0))
  (bind _asplayer_als_character (cast `/Game/AdvancedLocomotionV4/Blueprints/CharacterLogic/PlayerAlsCharacter` (`GameplayStatics.GetPlayerPawn` 0) :!pure true))
  (bind _output_get (set `self.IsPlayerInteract` (not (`self.IsPlayerInteract`))))
  (if _output_get
    (`/Game/AdvancedLocomotionV4/Blueprints/CharacterLogic/PlayerAlsCharacter.SetCustomCamera` _asplayer_als_character (`SceneComponent.K2_GetComponentToWorld` (`self.CameraRoot`)))
    (`self.DisableInput` _asplayer_als_character _returnvalue_2)
    (`self.EnableInput` _returnvalue_2)
    (`SceneComponent.SetVisibility` (`self.Interactable`) false true)
    (else
      (`/Game/AdvancedLocomotionV4/Blueprints/CharacterLogic/PlayerAlsCharacter.BackToNormalCamera` _asplayer_als_character)
      (`self.DisableInput` _returnvalue)
      (`self.EnableInput` _asplayer_als_character _returnvalue)
      (`SceneComponent.SetVisibility` (`self.Interactable`) true true))))

(event `Key|LeftMouseButton`
  (params (Key :type "Key Structure"))
  (bind (_hitresult _returnvalue) (`PlayerController.GetHitResultUnderCursorForObjects` (`GameplayStatics.GetPlayerController` 0) (`|MakeArray` "ObjectTypeQuery1" :!type "EObjectTypeQuery Enum") true))
  (bind (_bblockinghit _binitialoverlap _time _distance _location _impactpoint _normal _impactnormal _physmat _hitactor _hitcomponent) (`GameplayStatics.BreakHitResult` _hitresult))
  (:`Pressed`
    (if _returnvalue
      (if (`ActorComponent.ComponentHasTag` _hitcomponent "CodeButton")
        (`self.InputCode` (`KismetSystemLibrary.GetObjectName` _hitcomponent))))))

(event `InputAction|Use`
  (params (Key :type "Key Structure"))
  (:`Pressed`
    (`self.InteractWithObject`)))

(fn `InputCode`
  (params (Number :type String)))

(fn `UserConstructionScript`)