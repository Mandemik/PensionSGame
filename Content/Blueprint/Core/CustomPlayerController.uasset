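; Player controller that routes gameplay input actions to the third-person pawn.
; Reload, Distract and Attack presses call the pawn's fire-weapon reload, whistle and attack functions, while Inventory toggles the pawn's InventoryComponent.
; The controller only forwards input through its ThirdPersonPawn reference, which this graph never assigns or validity-checks.
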(event `InputAction|Reload`
  (params (Key :type "Key Structure"))
  (:`Pressed`
    (`/Game/ThirdPersonBP/Blueprints/ThirdPersonCharacter.ReloadFireWeapon` (`self.ThirdPersonPawn`))))

(event `InputAction|Distract`
  (params (Key :type "Key Structure"))
  (:`Pressed`
    (`/Game/ThirdPersonBP/Blueprints/ThirdPersonCharacter.Whistle` (`self.ThirdPersonPawn`))))

(event `InputAction|Attack`
  (params (Key :type "Key Structure"))
  (:`Pressed`
    (`/Game/ThirdPersonBP/Blueprints/ThirdPersonCharacter.Attack` (`self.ThirdPersonPawn`))))

(event `InputAction|Inventory`
  (params (Key :type "Key Structure"))
  (:`Pressed`
    (`/Game/Blueprint/Inventory/InventoryComponent.ToggleInventory` (`/Game/ThirdPersonBP/Blueprints/ThirdPersonCharacter.InventoryComponent` (`self.ThirdPersonPawn`)))))

(fn `UserConstructionScript`)