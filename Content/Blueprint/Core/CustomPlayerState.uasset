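; CustomPlayerState is a player state that tracks the player's weapon list, selected weapon index and ammo for Glock and Shotgun.
; Next and previous selection step the index within list bounds, print it, and have the ThirdPersonCharacter pawn set up that weapon class.
; Ammo functions compare the current weapon class to Glock or Shotgun to write magazine ammo or read and write equipment ammo in per-weapon variables.
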(fn `GetAmmoFromCurrentWeapon`
  (returns (PlayerAmmo :type Integer))
  (bind _output (`|GetArrayItem` (`self.WeaponList`) (`self.CurrentWeaponNumberList`)))
  (if (== _output "/Game/Blueprint/Weapon/Glock.Glock_C")
    (return (`self.GlockAmmoInEquipment`))
    (elif (== _output "/Game/Blueprint/Weapon/Shotgun.Shotgun_C")
      (return (`self.ShotgunAmmoInEquipment`)))))

(fn `SelectNextWeapon`
  (bind _currentweaponnumberlist (`self.CurrentWeaponNumberList`))
  (if (< (`self.CurrentWeaponNumberList`) (- (`KismetArrayLibrary.Array_Length` (`self.WeaponList`)) 1))
    (bind _result (`/Engine/EditorBlueprintResources/StandardMacros.IncrementInt` _currentweaponnumberlist)
      (:`  `
        (`KismetSystemLibrary.PrintString` (`KismetStringLibrary.Conv_IntToString` _currentweaponnumberlist))
        (`/Game/ThirdPersonBP/Blueprints/ThirdPersonCharacter.SetUpWeaponFromClass` (cast `/Game/ThirdPersonBP/Blueprints/ThirdPersonCharacter` (`self.PawnPrivate`) :!pure true) (`|GetArrayItem` (`self.WeaponList`) _result))))))

(fn `SelectPreviousWeapon`
  (if (> (`self.CurrentWeaponNumberList`) 0)
    (bind _result (`/Engine/EditorBlueprintResources/StandardMacros.DecrementInt` (`self.CurrentWeaponNumberList`))
      (:`  `
        (`KismetSystemLibrary.PrintString` (`KismetStringLibrary.Conv_IntToString` _result))
        (`/Game/ThirdPersonBP/Blueprints/ThirdPersonCharacter.SetUpWeaponFromClass` (cast `/Game/ThirdPersonBP/Blueprints/ThirdPersonCharacter` (`self.PawnPrivate`) :!pure true) (`|GetArrayItem` (`self.WeaponList`) _result))))))

(fn `SetAmmoInEquipmentAtCurrentWeapon`
  (params (Ammo :type Integer))
  (bind _output (`|GetArrayItem` (`self.WeaponList`) (`self.CurrentWeaponNumberList`)))
  (if (== _output "/Game/Blueprint/Weapon/Glock.Glock_C")
    (set `self.GlockAmmoInEquipment` Ammo)
    (elif (== _output "/Game/Blueprint/Weapon/Shotgun.Shotgun_C")
      (set `self.ShotgunAmmoInEquipment` Ammo))))

(fn `SetAmmoInMagAtCurrentWeapon`
  (params (AmmoInMag :type Integer))
  (bind _output (`|GetArrayItem` (`self.WeaponList`) (`self.CurrentWeaponNumberList`)))
  (if (== _output "/Game/Blueprint/Weapon/Glock.Glock_C")
    (set `self.GlockAmmoInMag` AmmoInMag)
    (elif (== _output "/Game/Blueprint/Weapon/Shotgun.Shotgun_C")
      (set `self.ShotgunAmmoInMag` AmmoInMag))))

(fn `UserConstructionScript`)