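; BasicAI is an enemy character with a Glock that can shoot, melee, crouch into cover and report danger with a debug print.
; BeginPlay links the GlockComponent to the weapon child actor's fire point and disables that actor's collision.
; StartShoot and StopShoot control a looping timer, guarded against restarts, for firing along the weapon's forward vector while alive.
; CharacterDie is empty; the ragdoll and controller death logic is disconnected.
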(event `self.ReceiveBeginPlay`
  (bind _glockcomponent (`self.GlockComponent`))
  (bind _childactor (`ChildActorComponent.ChildActor` (`self.Weapon`)))
  (set `/Game/Blueprint/Weapon/FireWeaponComponent.Owner` self _glockcomponent)
  (`self.SetActorEnableCollision` _childactor false)
  (set `/Game/Blueprint/Weapon/FireWeaponComponent.FireStart` (`/Game/Blueprint/Weapon/FireWeapon.FireStart` (cast `/Game/Blueprint/Weapon/Glock` _childactor :!pure true)) _glockcomponent))

(event `/Game/Blueprint/Core/CombatInterace.MeleeAttack`
  (`|PlayMontage` (`self.Mesh`) "/Game/Anim/Attack_PrimaryA_Montage.Attack_PrimaryA_Montage"))

(event `Threatened`
  (`KismetSystemLibrary.PrintString` "I am in danger"))

(event `CharacterDie`)

(event `/Game/Blueprint/Core/CombatInterace.StartShoot`
  (`self.StartShooting` (`|CreateDelegate` :!event `ShootingSequence`)))

(event `ShootingSequence`
  (bind _weapon (`self.Weapon`))
  (if (`self.IsLive`)
    (`/Game/Blueprint/Weapon/FireWeaponComponent.Fire` (`self.GlockComponent`) (+ (`SceneComponent.K2_GetComponentLocation` _weapon) (* (`KismetMathLibrary.GetForwardVector` (`SceneComponent.K2_GetComponentRotation` _weapon)) 10000.0)))))

(event `/Game/Blueprint/Core/CombatInterace.StopShoot`
  (`self.StopShooting`))

(event `EnterCover`
  (set `self.IsInCover` true)
  (`self.Crouch`))

(fn `StartShooting`
  (params (InputPin :type Delegate))
  (if (not (`self.EnemyShooting`))
    (set `self.EnemyShooting` true)
    (bind _returnvalue (`KismetSystemLibrary.K2_SetTimerDelegate` InputPin (`self.ShootFrequence`) true))
    (set `self.ShootingFrequenceTimer` _returnvalue)))

(fn `StopShooting`
  (set `self.EnemyShooting` false)
  (`KismetSystemLibrary.K2_ClearAndInvalidateTimerHandle` (`self.ShootingFrequenceTimer`)))

(fn `UserConstructionScript`)