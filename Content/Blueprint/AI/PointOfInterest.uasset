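; AI point of interest that drives social behavior among a list of bots, currently handling the Talking type.
; On BeginPlay it runs PlaySocialAnimation, which advances a wrapping index through the bot list in round-robin order.
; The selected bot's ALS_AI_Controller is told to start talking, then a non-looping timer is set to pace the conversation.
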(event `self.ReceiveBeginPlay`
  (`self.PlaySocialAnimation`))

(event `PlaySocialAnimation`
  (bind _listofbots (`self.ListOfBots`))
  (bind _activebotnumer (`self.ActiveBotNumer`))
  (switch `/Game/Blueprint/AI/IdleAnimationType` (`self.Type`)
    (:`NewEnumerator1`
      (if (>= _activebotnumer (- (`KismetArrayLibrary.Array_Length` _listofbots) 1))
        (set `self.ActiveBotNumer` 0)
        (else
          (`/Engine/EditorBlueprintResources/StandardMacros.IncrementInt` _activebotnumer
            (:`  `
              _))))
      (`/Game/AdvancedLocomotionV4/Blueprints/CharacterLogic/AI/ALS_AI_Controller.StartTalking` (cast `/Game/AdvancedLocomotionV4/Blueprints/CharacterLogic/AI/ALS_AI_Controller` (`Pawn.GetController` (`|GetArrayItem` _listofbots (`self.ActiveBotNumer`))) :!pure true))
      (`KismetSystemLibrary.K2_SetTimerDelegate` (`|CreateDelegate` :!event `PlaySocialAnimation`) 10.0))))

(fn `UserConstructionScript`)