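; Shotgun weapon Blueprint, a child that extends a parent weapon's firing with a pump animation.
; Fire calls the parent and, on success, triggers a timeline that moves the WeaponPump component along its relative Y axis.
; SetAmmoInMag calls the parent, then returns the shotgun magazine count read from player 0's ThirdPersonCharacter State.
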(event `PlayPumpUpAnimation`
  (bind _weaponpump (`self.WeaponPump`))
  (bind (_relativelocation_x _relativelocation_y _relativelocation_z) (`KismetMathLibrary.BreakVector` (`SceneComponent.RelativeLocation` _weaponpump)))
  (bind (_direction _newtrack_0) (`Timeline|PumpUpAnim` :!via `PlayFromStart`)
    (:`Update`
      (`SceneComponent.K2_SetRelativeLocation` _weaponpump (`KismetMathLibrary.MakeVector` _relativelocation_x _newtrack_0 _relativelocation_z) false false))))

(fn `Fire`
  (params (AimPoint :type "Vector Structure"))
  (returns (Sucseed :type Boolean) (CurrentMagAmmo :type Integer))
  (bind (_sucseed _currentmagammo) (`parent.Fire` AimPoint))
  (if _sucseed
    (`self.PlayPumpUpAnimation`))
  (return _sucseed _currentmagammo))

(fn `SetAmmoInMag`
  (returns (AmmoInMag :type Integer))
  (`parent.SetAmmoInMag`)
  (return (`/Game/Blueprint/Core/CustomPlayerState.ShotgunAmmoInMag` (`/Game/ThirdPersonBP/Blueprints/ThirdPersonCharacter.State` (cast `/Game/ThirdPersonBP/Blueprints/ThirdPersonCharacter` (`GameplayStatics.GetPlayerPawn` 0) :!pure true)))))

(fn `UserConstructionScript`
  (`parent.UserConstructionScript`))