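; Glock weapon component whose alternative use attaches or removes a silencer.
; AlternativeUse blocks shooting, plays the silencer montage on the owner's mesh, and only on completion re-enables shooting and flips the silencer state.
; The toggle swaps the fire sound and adds or removes the silencer mesh at the owner's suppressor socket.
; CheakSpecialFunction extends the parent's version to reapply sound and mesh from the current silencer state.
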(event `self.AlternativeUse`
  (`parent.AlternativeUse`)
  (set `self.CannotShot?` true)
  (`|PlayMontage` (`Character.Mesh` (`self.Owner`)) (`self.SilencerAnimation`)
    (:`OnCompleted`
      (set `self.CannotShot?` false)
      (if (`self.SillencerOn?`)
        (set `self.SillencerOn?` false)
        (set `self.FireSound` (`self.WithoutSilencerSound`))
        (`/Game/AdvancedLocomotionV4/Blueprints/CharacterLogic/ALS_AnimMan_CharacterBP.RemoveCustomToWeapon` (`self.Owner`) (`self.SilencerMesh`))
        (else
          (set `self.SillencerOn?` true)
          (set `self.FireSound` (`self.SilencerSound`))
          (`/Game/AdvancedLocomotionV4/Blueprints/CharacterLogic/ALS_AnimMan_CharacterBP.AddCustomToWeapon` (`self.Owner`) (`self.SilencerMesh`) "SuppressorSocket"))))))

(fn `CheakSpecialFunction`
  (`parent.CheakSpecialFunction`)
  (if (`self.SillencerOn?`)
    (set `self.FireSound` (`self.SilencerSound`))
    (`/Game/AdvancedLocomotionV4/Blueprints/CharacterLogic/ALS_AnimMan_CharacterBP.AddCustomToWeapon` (`self.Owner`) (`self.SilencerMesh`) "SuppressorSocket")
    (else
      (set `self.FireSound` (`self.WithoutSilencerSound`))
      (`/Game/AdvancedLocomotionV4/Blueprints/CharacterLogic/ALS_AnimMan_CharacterBP.RemoveCustomToWeapon` (`self.Owner`) (`self.SilencerMesh`)))))