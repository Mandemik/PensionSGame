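; Firearm item Blueprint that adds its class to the player's weapon list on use and handles firing and magazine ammo.
; Fire spends a round, then multi-sphere-traces from FireStart to the aim point, spawning explosion effects at hits.
; Non-simulating BasicAI hits die and receive radial force, as do physics-simulating hits.
; Reload refills the magazine and returns leftover ammo, syncing the count to the owner's State as Fire does.
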(event `self.ReceiveBeginPlay`)

(fn `Fire`
  (params (AimPoint :type "Vector Structure"))
  (returns (Sucseed :type Boolean) (CurrentMagAmmo :type Integer))
  (bind _currentammoinmag (`self.CurrentAmmoInMag`))
  (if (!= _currentammoinmag 0)
    (`GameplayStatics.PlaySoundAtLocation` (`self.FireSound`) (`self.K2_GetActorLocation`) (struct) 1.0 1.0 0.0 null null null)
    (bind _result (`/Engine/EditorBlueprintResources/StandardMacros.DecrementInt` (`self.CurrentAmmoInMag`))
      (:`  `
        (`/Game/Blueprint/Core/CustomPlayerState.SetAmmoInMagAtCurrentWeapon` (`/Game/ThirdPersonBP/Blueprints/ThirdPersonCharacter.State` (`self.CharacterOwner`)) _result)
        (bind (_outhits _returnvalue) (`KismetSystemLibrary.SphereTraceMultiForObjects` (`SceneComponent.K2_GetComponentLocation` (`self.FireStart`)) AimPoint (`self.FireRadius`) (`|MakeArray` "ObjectTypeQuery4" "ObjectTypeQuery2" "ObjectTypeQuery1" "ObjectTypeQuery3" :!type "EObjectTypeQuery Enum") true (`|MakeArray` (`GameplayStatics.GetPlayerPawn` 0) :!type "Actor Object Reference")))
        (`|ExecutionSequence`
          (:`then_0`
            (if _returnvalue
              (for _array_element _outhits
                (`|ExecutionSequence`
                  (:`then_0`
                    (bind (_bblockinghit _binitialoverlap _time _distance _location _impactpoint _normal _impactnormal _physmat _hitactor _hitcomponent) (`GameplayStatics.BreakHitResult` _array_element))
                    (if (not (`SceneComponent.IsSimulatingPhysics` _hitcomponent "None"))
                      (bind _asbasic_ai (cast `/Game/Blueprint/AI/BasicAI` _hitactor))
                      (`/Game/Blueprint/AI/BasicAI.CharacterDie` _asbasic_ai))
                    (`PrimitiveComponent.AddRadialForce` _hitcomponent _impactpoint 1000.0 1000000.0 "RIF_Constant" false))
                  (:`then_1`
                    (`GameplayStatics.SpawnEmitterAtLocation` "/Game/StarterContent/Particles/P_Explosion.P_Explosion" _impactpoint (struct) (0.1 0.1 0.1)))
                  (:`then_2`
                    (`KismetSystemLibrary.PrintString` (`KismetSystemLibrary.GetObjectName` _hitactor)))))
              (else
                (`KismetSystemLibrary.PrintString` "Hello"))))
          (:`then_1`
            (return true (`self.CurrentAmmoInMag`))))))
    (else
      (return false _currentammoinmag))))

(fn `InitWeapon`
  (params (CharacterOwner :type "/Game/ThirdPersonBP/Blueprints/ThirdPersonCharacter Object Reference"))
  (set `self.CharacterOwner` CharacterOwner)
  (bind _ammoinmag (`self.SetAmmoInMag`))
  (set `self.CurrentAmmoInMag` _ammoinmag))

(fn `Reload`
  (params (GetAmmo :type Integer))
  (returns (AmmoLeft :type Integer))
  (locals (PlayerAmmo :type Integer :default 0))
  (bind _state (`/Game/ThirdPersonBP/Blueprints/ThirdPersonCharacter.State` (`self.CharacterOwner`)))
  (bind _output_get (set `local.PlayerAmmo` (+ GetAmmo (`self.CurrentAmmoInMag`))))
  (if (<= _output_get (`self.MaxAmmoInMag`))
    (bind _output_get_2 (set `self.CurrentAmmoInMag` (`local.GetAmmo`)))
    (`/Game/Blueprint/Core/CustomPlayerState.SetAmmoInMagAtCurrentWeapon` _state _output_get_2)
    (return 0)
    (else
      (bind _output_get_3 (set `self.CurrentAmmoInMag` (`self.MaxAmmoInMag`)))
      (`/Game/Blueprint/Core/CustomPlayerState.SetAmmoInMagAtCurrentWeapon` _state _output_get_3)
      (return (- (`local.PlayerAmmo`) _output_get_3)))))

(fn `SetAmmoInMag`
  (returns (AmmoInMag :type Integer))
  (return 0))

(fn `UseItem`
  (returns (Success :type Boolean))
  (bind _returnvalue (`GameplayStatics.GetObjectClass` self))
  (`parent.UseItem`)
  (bind _asthird_person_character (cast `/Game/ThirdPersonBP/Blueprints/ThirdPersonCharacter` (`GameplayStatics.GetPlayerCharacter` 0)))
  (bind _weaponlist (`/Game/Blueprint/Core/CustomPlayerState.WeaponList` (`/Game/ThirdPersonBP/Blueprints/ThirdPersonCharacter.State` _asthird_person_character)))
  (if (not (`KismetArrayLibrary.Array_Contains` _weaponlist _returnvalue))
    (`KismetArrayLibrary.Array_Add` _weaponlist _returnvalue)
    (return true)))

(fn `UserConstructionScript`)

(fn `WeaponReloaded`
  (set `self.CurrentAmmoInMag` (`self.AmmoInReload`))
  (set `self.AmmoInReload` 0))