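; LightSwitch is an actor Blueprint that turns a group of lamps on and off when used.
; On BeginPlay it gathers every LightBulb component from the actors in ObjectWithLamp into a cached list.
; Each Use event flips the SwitchOn state and calls SwitchOn or SwitchOff on every cached bulb to match.
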(event `self.ReceiveBeginPlay`
  (for _array_element (`self.ObjectWithLamp`)
    (for _array_element_2 (`self.K2_GetComponentsByClass` _array_element "/Game/Blueprint/Actors/LightBulb.LightBulb_C")
      (`KismetArrayLibrary.Array_Add` (`self.LightBuldList`) _array_element_2))))

(event `/Game/Blueprint/Core/PlayerInteractive.Use`
  (bind _lightbuldlist (`self.LightBuldList`))
  (bind _output_get (set `self.SwitchOn` (not (`self.SwitchOn`))))
  (if _output_get
    (for _array_element _lightbuldlist
      (`/Game/Blueprint/Actors/LightBulb.SwitchOn` _array_element))
    (else
      (for _array_element_2 _lightbuldlist
        (`/Game/Blueprint/Actors/LightBulb.SwitchOff` _array_element_2)))))

(fn `UserConstructionScript`)