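; Inventory component that stores items in a fixed number of slots and toggles a centre-anchored inventory window on the player HUD, switching input mode and cursor.
; PrepareInventory sizes the array and refreshes item data from class defaults on BeginPlay and window open.
; AddToInventory tops up partial stacks, recursing on overflow, or fills an empty slot; UseOnAdd items are spawned and used.
; InventoryQuery checks whether an item's summed quantity meets a requested amount.
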(event `self.ReceiveBeginPlay`
  (`self.PrepareInventory`))

(fn `AddToInventory`
  (params (ContentToAdd :type "/Game/Blueprint/Inventory/SlotStructure Structure"))
  (returns (Success :type Boolean))
  (locals (IsSuccessful :type Boolean))
  (bind _contenttoadd (`local.ContentToAdd`))
  (`|ExecutionSequence`
    (:`then_0`
      (if (`.IsStackable_15_42A5D1844DA83681B81240BCB22480A1` (break `/Game/Blueprint/Inventory/ItemStructure` (break `/Game/Blueprint/Inventory/SlotStructure` ContentToAdd)))
        (bind _stackindex (`self.HasPartialStack` (`local.ContentToAdd`))
          (:`True`
            (bind _success (`self.AddToStack` (`local.ContentToAdd`) _stackindex))
            (set `local.IsSuccessful` _success))
          (:`False`
            (bind _success_2 (`self.CreateStack` (`local.ContentToAdd`) :!label _label))
            (set `local.IsSuccessful` _success_2)))
        (else
          (goto _label)))
      (if (`.UseOnAdd_24_64C9431049E4058863B4B0BF365CC8B3` (break `/Game/Blueprint/Inventory/ItemStructure` (break `/Game/Blueprint/Inventory/SlotStructure` _contenttoadd)))
        (for _ (range 1 (+ (`.Quanitli_5_C21ADFDA49204B1E16762189682E6CF9` (break `/Game/Blueprint/Inventory/SlotStructure` _contenttoadd)) 1))
          (bind _returnvalue (`|SpawnActorFromClass` (`.Class_22_E0FD0612400E999F6B2D0482BFF6E503` (break `/Game/Blueprint/Inventory/ItemStructure` (break `/Game/Blueprint/Inventory/SlotStructure` _contenttoadd))) (`KismetMathLibrary.MakeTransform` (0.0 0.0 0.0) (struct) (0.0 0.0 0.0)) "Undefined" "OverrideRootScale" null null))
          (`/Game/Blueprint/Inventory/Item/Item.UseItem` _returnvalue))))
    (:`then_1`
      (return (`local.IsSuccessful`)))))

(fn `AddToStack`
  (params (SlotStructure :type "/Game/Blueprint/Inventory/SlotStructure Structure") (SlotIndex :type Integer))
  (returns (Success :type Boolean))
  (locals (CurrentQuantity :type Integer))
  (bind _slotindex (`local.SlotIndex`))
  (bind (_slotstructure_itemstructure _slotstructure_quanitli) (break `/Game/Blueprint/Inventory/SlotStructure` (`local.SlotStructure`)))
  (bind _inventory (`self.Inventory`))
  (bind (_slotstructure_itemstructure_2 _slotstructure_quanitli_2) (break `/Game/Blueprint/Inventory/SlotStructure` (`local.SlotStructure`)))
  (bind _slotstructure_itemstructure_3 (break `/Game/Blueprint/Inventory/SlotStructure` (`local.SlotStructure`)))
  (bind (_name _isstackable _thumbrail _maxstacksize) (break `/Game/Blueprint/Inventory/ItemStructure` _slotstructure_itemstructure_3))
  (bind _output (`|GetArrayItem` (`self.Inventory`) SlotIndex))
  (bind (_output_itemstructure _output_quanitli) (break `/Game/Blueprint/Inventory/SlotStructure` (`|GetArrayItem` _inventory _slotindex)))
  (bind _output_get (set `local.CurrentQuantity` (`.Quanitli_5_C21ADFDA49204B1E16762189682E6CF9` (break `/Game/Blueprint/Inventory/SlotStructure` _output))))
  (if (> (+ _output_get (`.Quanitli_5_C21ADFDA49204B1E16762189682E6CF9` (break `/Game/Blueprint/Inventory/SlotStructure` SlotStructure))) (`.MaxStackSize_17_8510A6DA4ECAFE50B1EAA8B38D5C9E30` (break `/Game/Blueprint/Inventory/ItemStructure` (break `/Game/Blueprint/Inventory/SlotStructure` _output))))
    (`KismetArrayLibrary.Array_Set` (`self.Inventory`) (`local.SlotIndex`) (make `/Game/Blueprint/Inventory/SlotStructure` _slotstructure_itemstructure_3 _maxstacksize))
    (`self.AddToInventory` (make `/Game/Blueprint/Inventory/SlotStructure` _slotstructure_itemstructure (- _slotstructure_quanitli (- _maxstacksize (`local.CurrentQuantity`)))))
    (else
      (`KismetArrayLibrary.Array_Set` _inventory _slotindex (make `/Game/Blueprint/Inventory/SlotStructure` _output_itemstructure (+ _output_quanitli _slotstructure_quanitli_2)))))
  (return true))

(fn `BindToPlayerCamera`)

(fn `CreateStack`
  (params (ContentToAdd :type "/Game/Blueprint/Inventory/SlotStructure Structure"))
  (returns (Success :type Boolean))
  (locals (HasSpace :type Boolean))
  (bind _inventory (`self.Inventory`))
  (for _array_element (`self.Inventory`)
    (if (<= (`.Quanitli_5_C21ADFDA49204B1E16762189682E6CF9` (break `/Game/Blueprint/Inventory/SlotStructure` _array_element)) 0)
      (set `local.HasSpace` true)
      (break)))
  (if (`local.HasSpace`)
    (`KismetArrayLibrary.Array_Set` _inventory (`KismetArrayLibrary.Array_Find` _inventory (make `/Game/Blueprint/Inventory/SlotStructure` (struct :`Name` "NSLOCTEXT(\"[35D51D2E40BDB1109C1A5F98720565D0]\", \"864ADB8E4DA524BA4E00B2B47CE58A14\", \"None\")" :`IsStackable` true :`MaxStackSize` 4 :`IsConsumable` true :`Description` "NSLOCTEXT(\"[35D51D2E40BDB1109C1A5F98720565D0]\", \"3675B1B24D2DE6004BA55F8CCA0CB8AB\", \"None\")"))) (`local.ContentToAdd`))
    (return (`local.HasSpace`))
    (else
      (return false))))

(fn `InventoryQuery`
  (params (QueryItem :type "/Game/Blueprint/Inventory/Item/Item Class Reference") (QueryAmont :type Integer))
  (returns (IsInInventory :type Boolean))
  (locals (RunningTotal :type Integer))
  (for _array_element (`self.Inventory`)
    (if (== (`.Class_22_E0FD0612400E999F6B2D0482BFF6E503` (break `/Game/Blueprint/Inventory/ItemStructure` (break `/Game/Blueprint/Inventory/SlotStructure` _array_element))) (`local.QueryItem`))
      (set `local.RunningTotal` (+ (`.Quanitli_5_C21ADFDA49204B1E16762189682E6CF9` (break `/Game/Blueprint/Inventory/SlotStructure` _array_element)) (`local.RunningTotal`)))))
  (return (>= (`local.RunningTotal`) (`local.QueryAmont`))))

(fn `PrepareInventory`
  (`KismetArrayLibrary.Array_Resize` (`self.Inventory`) (`self.NumberOfSlots`))
  (for (_array_element _array_index) (`self.Inventory`)
    (bind (_name _isstackable _thumbrail _maxstacksize _isconsumable _duration _description _class) (break `/Game/Blueprint/Inventory/ItemStructure` (break `/Game/Blueprint/Inventory/SlotStructure` _array_element)))
    (if (!= _class null)
      (`KismetArrayLibrary.Array_Set` (`self.Inventory`) _array_index (make `/Game/Blueprint/Inventory/SlotStructure` (defaults `/Game/Blueprint/Inventory/InventoryComponent` _class) (`.Quanitli_5_C21ADFDA49204B1E16762189682E6CF9` (break `/Game/Blueprint/Inventory/SlotStructure` _array_element)))))))

(fn `ToggleInventory`
  (bind _returnvalue (`GameplayStatics.GetPlayerController` 0))
  (bind _inventorywindow (`self.InventoryWindow`)
    (:`then`
      (`Widget.RemoveFromParent` _inventorywindow)
      (set `self.InventoryWindow` null)
      (`WidgetBlueprintLibrary.SetInputMode_GameOnly` (`GameplayStatics.GetPlayerController` 0))
      (set `PlayerController.bShowMouseCursor` false (`GameplayStatics.GetPlayerController` 0))
      (`self.InventoryToggle` false)
      (clear `self.InventoryToggle`))
    (:`else`
      (`self.PrepareInventory`)
      (bind _returnvalue_2 (`|CreateWidget` "/Game/Blueprint/WidgetsBP/Inventory/InventoryWindow.InventoryWindow_C" null self))
      (set `self.InventoryWindow` _returnvalue_2)
      (bind _returnvalue_3 (`CanvasPanel.AddChildToCanvas` (`/Game/Blueprint/WidgetsBP/HUD/PlayerHudContainer.CanvasPanel_0` (`/Game/AdvancedLocomotionV3/Blueprints/ALS_BaseCharacter.PlayerHUD` (cast `/Game/AdvancedLocomotionV3/Blueprints/MannequinCharacter` (`GameplayStatics.GetPlayerPawn` 0) :!pure true))) (`self.InventoryWindow`)))
      (`CanvasPanelSlot.SetAutoSize` _returnvalue_3 true)
      (`CanvasPanelSlot.SetAlignment` _returnvalue_3 (0.5 0.5))
      (`CanvasPanelSlot.SetAnchors` _returnvalue_3 (make `Anchors` (0.5 0.5) (0.5 0.5)))
      (`CanvasPanelSlot.SetPosition` _returnvalue_3 (`self.Position`))
      (`WidgetBlueprintLibrary.SetInputMode_UIOnlyEx` _returnvalue (`self.InventoryWindow`) "LockAlways")
      (set `PlayerController.bShowMouseCursor` true _returnvalue)
      (`self.InventoryToggle` true))))