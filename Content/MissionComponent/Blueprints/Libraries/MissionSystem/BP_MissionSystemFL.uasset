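; Blueprint function library for the mission system, giving helpers to reach the local player's mission component and query mission, objective and target state.
; The component comes via a RequestMissionComponentMessage call on player controller 0 or an overlapping pawn's controller, gated by local-control checks.
; Mission queries read that component, while target lookups search the level's BP_TargetsManager by unique name, printing a warning if it is missing.
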(fn `FindInCurrentTargets`
  (params (WithUniqueName :type Name))
  (returns (TargetInfo :type "/Game/MissionComponent/Blueprints/Structs/MissionComponent/Struct_TargetInfo Structure"))
  (locals (LocTargetInfo :type "/Game/MissionComponent/Blueprints/Structs/MissionComponent/Struct_TargetInfo Structure"))
  ;[0 0 0 1 16] Search For Each Loop With Same Unique Name
  (for _array_element (`/Game/MissionComponent/Blueprints/Manager/BP_TargetsManager.Targets` (`self.GetTargetManager` null))
    (if (== (`.TargetUniqueName_7_FE44C2044550DF171469159B30339FAA` (break `/Game/MissionComponent/Blueprints/Structs/MissionComponent/Struct_TargetInfo` _array_element)) WithUniqueName)
      (set `local.LocTargetInfo` _array_element)
      (break)
      (else
        (set `local.LocTargetInfo` (struct)))))
  (return (`local.LocTargetInfo`)))

(fn `GetMissionComponent`
  (returns (ReturnValue :type "/Game/MissionComponent/Blueprints/Components/BP_MissionComponent Object Reference"))
  (locals (LocMissionComponent :type "/Game/MissionComponent/Blueprints/Components/BP_MissionComponent Object Reference"))
  (bind _returnvalue (`GameplayStatics.GetPlayerController` null))
  (bind _locmissioncomponent (`local.LocMissionComponent`))
  (bind _returnvalue_2 (`Controller.K2_GetPawn` _returnvalue))
  ;[0 0 0 1 16] Check If The Player Is Locally Controlled Or Not
  (`/Engine/EditorBlueprintResources/StandardMacros.IsValid` _returnvalue
    (:`Is Valid`
      (`/Engine/EditorBlueprintResources/StandardMacros.IsValid` _returnvalue_2
        (:`Is Valid`
          (if (and (`Pawn.IsLocallyControlled` _returnvalue_2) (`Pawn.IsControlled` _returnvalue_2))
            (bind _missioncomponent (message `/Game/MissionComponent/Blueprints/Interfaces/MissionSystem/BP_PlayerControllerInterface.RequestMissionComponent` (`GameplayStatics.GetPlayerController` null)))
            (set `local.LocMissionComponent` _missioncomponent)
            (`/Engine/EditorBlueprintResources/StandardMacros.IsValid` _locmissioncomponent
              (:`Is Valid`
                (return _locmissioncomponent))
              (:`Is Not Valid`
                (return null)))
            (else
              (return null))))
        (:`Is Not Valid`
          _)))
    (:`Is Not Valid`
      _))
  (return null))

(fn `GetTargetManager`
  (returns (Output :type "/Game/MissionComponent/Blueprints/Manager/BP_TargetsManager Object Reference"))
  (bind _outactors (`GameplayStatics.GetAllActorsOfClass` null "/Game/MissionComponent/Blueprints/Manager/BP_TargetsManager.BP_TargetsManager_C"))
  (bind _output (`|GetArrayItem` _outactors))
  (`/Engine/EditorBlueprintResources/StandardMacros.IsValid` _output
    (:`Is Valid`
      (return _output))
    (:`Is Not Valid`
      (`KismetSystemLibrary.PrintString` null "Add BP_TargetsManager To Your Persistent Level!" true true (struct :`R` 1.0 :`B` 0.00718 :`A` 1.0) 20.0)
      (return null))))

(fn `IsInMission?`
  (returns (ReturnValue :type Boolean))
  (locals (LocUniqueName :type Name))
  (return (`/Game/MissionComponent/Blueprints/Components/BP_MissionComponent.InMission?` (`self.GetMissionComponent` null))))

(fn `IsInSpecificMission?`
  (params (UniqueMissionName :type Name))
  (returns (ReturnValue :type Boolean))
  (locals (LocUniqueName :type Name))
  (bind _returnvalue (`self.GetMissionComponent` null))
  (set `local.LocUniqueName` UniqueMissionName)
  (`/Engine/EditorBlueprintResources/StandardMacros.IsValid` _returnvalue
    (:`Is Valid`
      (return (and (== (`local.LocUniqueName`) (`KismetStringLibrary.Conv_StringToName` (`KismetTextLibrary.Conv_TextToString` (`.Name_7_1EC463E048DAF608492E408397699B38` (break `/Game/MissionComponent/Blueprints/Structs/MissionComponent/Struct_MMainInfo` (`.MissionMainInfo_12_1EC463E048DAF608492E408397699B38` (break `/Game/MissionComponent/Blueprints/Structs/MissionComponent/Struct_MissionMaster` (`/Game/MissionComponent/Blueprints/Components/BP_MissionComponent.CurrentMission` _returnvalue)))))))) (`/Game/MissionComponent/Blueprints/Components/BP_MissionComponent.InMission?` _returnvalue))))))

(fn `IsLocalPawn`
  (params (Pawn :type "Actor Object Reference"))
  (returns (ReturnValue :type Boolean))
  (bind _aspawn (cast `Pawn` Pawn))
  (return (and (`Pawn.IsLocallyControlled` _aspawn) (`Pawn.IsControlled` _aspawn))))

(fn `IsTargetInCurrentObjectives`
  (params (TargetUniqueName :type Name))
  (returns (ReturnValue :type Boolean))
  (locals (LocUniqueName :type Name) (LocIsInObjectives :type Boolean :default false))
  (bind _returnvalue (`self.GetMissionComponent` null))
  (set `local.LocUniqueName` TargetUniqueName)
  (for _array_element (`/Game/MissionComponent/Blueprints/Components/BP_MissionComponent.CurrentObjectives` _returnvalue)
    (bind ((`ObjectiveClass_44_03513BF742C17DDC3C716E8FB39B5963` _objectiveclass) (`ObjectiveTargets_48_1F7C5F2E4E99CBB6A2D4398D5F5A1DA5` _objectivetargets)) (break `/Game/MissionComponent/Blueprints/Structs/MissionComponent/Struct_Objectives` _array_element))
    (switch `/Game/MissionComponent/Blueprints/Enums/MissionComponent/Enum_ObjectiveLType` _objectiveclass
      (:`NewEnumerator1`
        (if (== (`.TargetsUniqueName_14_1EC463E048DAF608492E408397699B38` (break `/Game/MissionComponent/Blueprints/Structs/MissionComponent/Struct_ObjectiveMainInfo` (`|GetArrayItem` _objectivetargets))) (`local.LocUniqueName`))
          (set `local.LocIsInObjectives` true)
          (else
            (set `local.LocIsInObjectives` false))))
      (:`NewEnumerator2`
        (for _array_element_2 _objectivetargets
          (if (== (`.TargetsUniqueName_14_1EC463E048DAF608492E408397699B38` (break `/Game/MissionComponent/Blueprints/Structs/MissionComponent/Struct_ObjectiveMainInfo` _array_element_2)) (`local.LocUniqueName`))
            (set `local.LocIsInObjectives` true)
            (break)
            (else
              (set `local.LocIsInObjectives` false)))))))
  (return (and (`local.LocIsInObjectives`) (`/Game/MissionComponent/Blueprints/Components/BP_MissionComponent.InMission?` _returnvalue))))

(fn `MissionComponentOnOverlap`
  (params (OtherActor :type "Actor Object Reference"))
  (returns (CanAccess :type Boolean) (ComponentReference :type "/Game/MissionComponent/Blueprints/Components/BP_MissionComponent Object Reference"))
  (locals (LocMissionComponent :type "/Game/MissionComponent/Blueprints/Components/BP_MissionComponent Object Reference"))
  (bind _locmissioncomponent (`local.LocMissionComponent`))
  ;[0 0 0 1 16] Check If The Player Is Locally Controlled Or Not
  (bind _aspawn (cast `Pawn` OtherActor)
    (:`then`
      (bind _returnvalue (`Pawn.GetController` _aspawn))
      (`/Engine/EditorBlueprintResources/StandardMacros.IsValid` _returnvalue
        (:`Is Valid`
          (bind _missioncomponent (message `/Game/MissionComponent/Blueprints/Interfaces/MissionSystem/BP_PlayerControllerInterface.RequestMissionComponent` _returnvalue))
          (set `local.LocMissionComponent` _missioncomponent)
          (if (and (`Controller.IsLocalController` _returnvalue) (`Controller.IsLocalPlayerController` _returnvalue))
            (`/Engine/EditorBlueprintResources/StandardMacros.IsValid` _locmissioncomponent
              (:`Is Valid`
                (return true _locmissioncomponent))
              (:`Is Not Valid`
                (return false null)))
            (else
              (return false null))))))
    (:`CastFailed`
      (return false null))))