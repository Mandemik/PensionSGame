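; SuspiciousZone is an overlap zone actor that shows an on-screen warning while something is inside it.
; Begin overlap creates a widget, adds it to the viewport, stores it as WarningWidget and sets SuspicionActivated; end overlap removes the widget and clears the flag.
; Overlaps are not filtered by actor, and each begin overlap overwrites the stored widget reference.
; Disconnected leftover nodes include a tag check and a level load that never run.
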(event `self.ReceiveBeginPlay`)

(event `self.ReceiveActorBeginOverlap`
  (params (OtherActor :type "Actor Object Reference"))
  (bind _returnvalue (`|CreateWidget` (`self.widgetClass`)))
  (`UserWidget.AddToViewport` _returnvalue 0)
  (set `self.WarningWidget` _returnvalue)
  (set `self.SuspicionActivated` true))

(event `self.ReceiveActorEndOverlap`
  (params (OtherActor :type "Actor Object Reference"))
  (`Widget.RemoveFromParent` (`self.WarningWidget`))
  (set `self.SuspicionActivated` false))

(fn `UserConstructionScript`)