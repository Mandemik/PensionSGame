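; DangerZone is a trigger actor that fails the level when a Character-tagged component enters its box while its child SuspiciousZone has suspicion activated.
; Being caught removes the zone's warning widget, disables player input and shows a Caught screen, replaced by a Failed screen two seconds later.
; Tick-driven gates then open to poll keys, letting the player reload Pensions_Level with Enter or quit the game.
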(event `self.ReceiveBeginPlay`
  (set `self.PostProc` (make `PostProcessSettings`)))

(event `Key|Enter`
  (params (Key :type "Key Structure")))

(event `self.ReceiveActorBeginOverlap`
  (params (OtherActor :type "Actor Object Reference")))

(event `self.Box.OnComponentBeginOverlap`
  (params (OverlappedComponent :type "PrimitiveComponent Object Reference") (OtherActor :type "Actor Object Reference") (OtherComp :type "PrimitiveComponent Object Reference") (OtherBodyIndex :type Integer) (bFromSweep :type Boolean) (SweepResult :type "HitResult Structure (by ref)"))
  (bind _returnvalue (`GameplayStatics.GetPlayerController` 0))
  (if (`ActorComponent.ComponentHasTag` OtherComp "Character")
    (bind _assuspicious_zone (cast `/Game/1Main/Blueprints/SuspiciousZone` (`ChildActorComponent.ChildActor` (`self.SuspiciousZone`))))
    (if (`/Game/1Main/Blueprints/SuspiciousZone.SuspicionActivated` _assuspicious_zone)
      (`Widget.RemoveFromParent` (`/Game/1Main/Blueprints/SuspiciousZone.WarningWidget` _assuspicious_zone))
      (bind _returnvalue_2 (`|CreateWidget` "/Game/1Main/Blueprints/Widgets/Caught.Caught_C"))
      (`UserWidget.AddToViewport` _returnvalue_2 0)
      (`self.DisableInput` (`GameplayStatics.GetPlayerCharacter` 0) (`GameplayStatics.GetPlayerController` 0))
      (`KismetSystemLibrary.Delay` 2.0)
      (`Widget.RemoveFromParent` _returnvalue_2)
      (bind _returnvalue_3 (`|CreateWidget` "/Game/1Main/Blueprints/Widgets/Failed.Failed_C"))
      (`UserWidget.AddToViewport` _returnvalue_3 0)
      (`|ExecutionSequence`
        (:`then_0`
          (goto _label :!via `Open`))
        (:`then_1`
          (goto _label_2 :!via `Open`))))))

(event `self.ReceiveTick`
  (params (DeltaSeconds :type "Float (single-precision)"))
  (bind _returnvalue (`GameplayStatics.GetPlayerController` 0))
  (`|ExecutionSequence`
    (:`then_0`
      (`/Engine/EditorBlueprintResources/StandardMacros.Gate` true :!label _label
        (:`Exit`
          (if (`PlayerController.WasInputKeyJustPressed` _returnvalue "Enter")
            (`GameplayStatics.OpenLevel` "Pensions_Level")))))
    (:`then_1`
      (`/Engine/EditorBlueprintResources/StandardMacros.Gate` true :!label _label_2
        (:`Exit`
          (if (or (`PlayerController.WasInputKeyJustPressed` _returnvalue "Escape") (`PlayerController.WasInputKeyJustPressed` _returnvalue "One"))
            (`KismetSystemLibrary.QuitGame` null "Quit")))))))

(event `Key|Escape`
  (params (Key :type "Key Structure")))

(event `Key|One`
  (params (Key :type "Key Structure")))

(fn `UserConstructionScript`)