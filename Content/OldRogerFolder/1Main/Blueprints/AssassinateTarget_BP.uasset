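; AssassinateTarget_BP is a mission objective trigger that lets the player assassinate a target by pressing Enter nearby.
; Box overlap with a Character-tagged component shows or removes the prompt widget and opens or closes a Gate on Tick that polls for the key.
; On the press, it swaps the prompt for a TargetAssassinated widget, flags EndMission_BP's IsTargetAssassinated, and removes the confirmation after a short delay.
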(event `self.ReceiveTick`
  (params (DeltaSeconds :type "Float (single-precision)"))
  (`/Engine/EditorBlueprintResources/StandardMacros.Gate` true :!label _label
    (:`Exit`
      (if (`PlayerController.WasInputKeyJustPressed` (`GameplayStatics.GetPlayerController` 0) "Enter")
        (bind _foundwidgets (`WidgetBlueprintLibrary.GetAllWidgetsOfClass` "/Game/1Main/Blueprints/Widgets/Player/AssassinateTarget.AssassinateTarget_C"))
        (`Widget.RemoveFromParent` (`|GetArrayItem` _foundwidgets))
        (bind _returnvalue (`|CreateWidget` "/Game/1Main/Blueprints/Widgets/Player/TargetAssassinated.TargetAssassinated_C"))
        (`UserWidget.AddToViewport` _returnvalue 0)
        (bind _outactors (`GameplayStatics.GetAllActorsOfClass` "/Game/1Main/Blueprints/EndMission_BP.EndMission_BP_C"))
        (set `/Game/1Main/Blueprints/EndMission_BP.IsTargetAssassinated` true (`|GetArrayItem` _outactors))
        (`KismetSystemLibrary.Delay` 5.0)
        (bind _foundwidgets_2 (`WidgetBlueprintLibrary.GetAllWidgetsOfClass` "/Game/1Main/Blueprints/Widgets/Player/TargetAssassinated.TargetAssassinated_C"))
        (`Widget.RemoveFromParent` (`|GetArrayItem` _foundwidgets_2))))))

(event `self.Box.OnComponentBeginOverlap`
  (params (OverlappedComponent :type "PrimitiveComponent Object Reference") (OtherActor :type "Actor Object Reference") (OtherComp :type "PrimitiveComponent Object Reference") (OtherBodyIndex :type Integer) (bFromSweep :type Boolean) (SweepResult :type "HitResult Structure (by ref)"))
  (if (`ActorComponent.ComponentHasTag` OtherComp "Character")
    (bind _returnvalue (`|CreateWidget` "/Game/1Main/Blueprints/Widgets/Player/AssassinateTarget.AssassinateTarget_C"))
    (`UserWidget.AddToViewport` _returnvalue 0)
    (goto _label :!via `Open`)))

(event `self.Box.OnComponentEndOverlap`
  (params (OverlappedComponent :type "PrimitiveComponent Object Reference") (OtherActor :type "Actor Object Reference") (OtherComp :type "PrimitiveComponent Object Reference") (OtherBodyIndex :type Integer))
  (if (`ActorComponent.ComponentHasTag` OtherComp "Character")
    (bind _foundwidgets (`WidgetBlueprintLibrary.GetAllWidgetsOfClass` "/Game/1Main/Blueprints/Widgets/Player/AssassinateTarget.AssassinateTarget_C"))
    (`Widget.RemoveFromParent` (`|GetArrayItem` _foundwidgets))
    (goto _label :!via `Close`)))

(fn `UserConstructionScript`)